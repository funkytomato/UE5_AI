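; BP_NPC is an AI character Blueprint with simple stance events for Cover, Advance, Retreat and Attack.
; Cover crouches the character, while Advance, Retreat and Attack stand it up; Attack only prints a debug message.
; Hit events are reported as touch events, with the NPC as receiver and the colliding actor and location passed along, for AI perception.
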(event `self.ReceiveBeginPlay`)

(event `self.ReceiveHit`
  (params (MyComp :type "PrimitiveComponent Object Reference") (Other :type "Actor Object Reference") (OtherComp :type "PrimitiveComponent Object Reference") (bSelfMoved :type Boolean) (HitLocation :type "Vector Structure") (HitNormal :type "Vector Structure") (NormalImpulse :type "Vector Structure") (Hit :type "HitResult Structure (by ref)"))
  (`AISense_Touch.ReportTouchEvent` self Other HitLocation))

(event `/Game/Characters/AI/I_Combat.Cover`
  (`self.Crouch`))

(event `/Game/Characters/AI/I_Combat.Advance`
  (`self.UnCrouch`))

(event `/Game/Characters/AI/I_Combat.Retreat`
  (`self.UnCrouch`))

(event `/Game/Characters/AI/I_Combat.Attack`
  (`self.UnCrouch`)
  (`KismetSystemLibrary.PrintString` "Attacking"))

(fn `UserConstructionScript`)